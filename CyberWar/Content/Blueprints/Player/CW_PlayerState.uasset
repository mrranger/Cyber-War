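; Player state holding a player's team, per-team character choice, weapon loadout, name and match kill/death tallies.
; Item IDs resolve to character meshes by team and to weapons by slot.
; RepNotifies push mesh and primary, secondary or melee changes to the owning CW_Character, found via its controller or an actor search.
; BaseState's RepNotify requests a name change through the game mode using player controller 0.
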(event `self.ReceiveBeginPlay`)

(fn `GetCharacterMesh`
  (returns (ChraracterMesh :type "/Game/Blueprints/Character/CW_CharacterMesh Class Reference"))
  (return (`/Game/Blueprints/Library/ItemFunctionLibrary.ItemToCharacterMesh` (`/Game/Blueprints/Library/ItemFunctionLibrary.GetItem` (`self.GetCharacterMeshID`)))))

(fn `GetCharacterMeshID`
  (returns (ReturnValue :type Integer))
  (return (select `/Game/Blueprints/Engine/ETeam` (`self.Team`) :`NewEnumerator0` (`self.C_Red`) :`NewEnumerator1` (`self.C_Blue`))))

(fn `GetSelectedWeapon`
  (params (Slot :type "/Game/Blueprints/Weapon/EWeaponSlot Enum" :default "NewEnumerator0"))
  (returns (Weapon :type "/Game/Blueprints/Weapon/Weapon Class Reference"))
  (locals (LocalWeapons :type "Array of /Game/Blueprints/Weapon/Weapon Class Reference"))
  (bind _weapon (`/Game/Blueprints/Library/ItemFunctionLibrary.ItemToWeapon` (`/Game/Blueprints/Library/ItemFunctionLibrary.GetItem` (select `/Game/Blueprints/Weapon/EWeaponSlot` Slot :`NewEnumerator0` (`self.W_Primary`) :`NewEnumerator1` (`self.W_Secondary`) :`NewEnumerator2` (`self.W_Melee`) :`NewEnumerator3` (`self.W_Throw`) :`NewEnumerator4` (`self.W_Special`)))))
  (`/Game/Blueprints/Library/ObjectMacroLibrary.IsValidClass` _weapon
    (:`Is Valid`
      (return _weapon))
    (:`Is Not Valid`
      (return null))))

(fn `IncrementDeaths`
  (set `self.MatchDeaths` (+ (`self.MatchDeaths`) 1))
  (return))

(fn `IncrementKills`
  (params (bWasTeamKill :type Boolean))
  (if bWasTeamKill
    (set `self.AlliesKilled` (+ (`self.AlliesKilled`) 1))
    (return)
    (else
      (set `self.RivalsKilled` (+ (`self.RivalsKilled`) 1))
      (return))))

(fn `OnRep_BaseState`
  (bind _basestate_name (break `/Game/Blueprints/Player/FPlayerModel` (`self.BaseState`)))
  (`GameModeBase.ChangeName` (`GameplayStatics.GetGameMode`) (`GameplayStatics.GetPlayerController` 0) _basestate_name true))

(fn `OnRep_C_Blue`
  (`self.UpdateCharacterMesh`))

(fn `OnRep_C_Red`
  (`self.UpdateCharacterMesh`))

(fn `OnRep_SelectedCharacterMeshBlue`
  (`self.UpdateCharacterMesh`)
  (return))

(fn `OnRep_SelectedCharacterMeshRed`
  (`self.UpdateCharacterMesh`)
  (return))

(fn `OnRep_Team`
  (`self.UpdateCharacterMesh`)
  (return))

(fn `OnRep_W_Melee`
  (`self.UpdateSelectedWeapon` "NewEnumerator2")
  (return))

(fn `OnRep_W_Primary`
  (`self.UpdateSelectedWeapon` "NewEnumerator0")
  (return))

(fn `OnRep_W_Secondary`
  (`self.UpdateSelectedWeapon` "NewEnumerator1")
  (return))

(fn `UpdateCharacterMesh`
  (bind _ascw_player_controller (cast `/Game/Blueprints/Player/CW_playerController` (`self.GetOwner`))
    (:`then`
      (bind _ascw_character (cast `/Game/Blueprints/Character/CW_Character` (`Controller.K2_GetPawn` _ascw_player_controller))
        (:`then`
          (`/Game/Blueprints/Character/CW_Character.UpdateCharacterMesh` _ascw_character))
        (:`CastFailed`
          (return))))
    (:`CastFailed`
      (bind _outactors (`GameplayStatics.GetAllActorsOfClass` "/Game/Blueprints/Character/CW_Character.CW_Character_C"))
      (for _array_element _outactors
        (if (== (`/Game/Blueprints/Character/CW_Character.CWPlayerState` _array_element) self)
          (`/Game/Blueprints/Character/CW_Character.UpdateCharacterMesh` _array_element)
          (break)))
      (return))))

(fn `UpdateSelectedWeapon`
  (params (Slot :type "/Game/Blueprints/Weapon/EWeaponSlot Enum" :default "NewEnumerator0"))
  (bind _outactors (`GameplayStatics.GetAllActorsOfClass` "/Game/Blueprints/Character/CW_Character.CW_Character_C"))
  (for _array_element _outactors
    (if (== (`/Game/Blueprints/Character/CW_Character.CWPlayerState` _array_element) self)
      (`/Game/Blueprints/Weapon/WeaponManager.OverrideSelecterWeapon` (`/Game/Blueprints/Character/CW_Character.WeaponManager` _array_element) Slot (`self.GetSelectedWeapon` Slot))
      (break)))
  (return))

(fn `UserConstructionScript`)